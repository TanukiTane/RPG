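; Character storage component that holds the rifle, weapon items and ammo, and manages the weapon in hand.
; A picked-up rifle attaches to a hide socket, and switching toggles it into the hand socket or drops the previous weapon ahead.
; The attach event briefly stops the character and delays the socket change.
; Ammo pickups stack by class, and a lookup returns the stack matching the current firearm's bullet type.
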(event Custom|Weapon%20Attach
  (params (Weapon :type BP%20Weapon%20Actor%20Object%20Reference) (SocketName :type Name))
  ;[1 1 1] Weapon Attach
  (Utilities|FlowControl|Sequence
    (:then_0
      (Variables|/Game/Blueprints/BP_MainChacter.BP_MainChacter_C|SetIsStopped (Variables|Default|GetCharacter) true)
      (Utilities|FlowControl|Delay 0.7)
      (CallFunction|WeaponAttach Weapon SocketName))
    (:then_1
      (Utilities|FlowControl|Delay 1.8)
      (Variables|/Game/Blueprints/BP_MainChacter.BP_MainChacter_C|SetIsStopped (Variables|Default|GetCharacter) false))))

(event Event-Init
  ;[1 1 1] Init
  (|CallParentFunction))

(fn WeaponAdd
  (params (Weapon :type BP%20Weapon%20Actor%20Object%20Reference))
  (bind _asbp_weapon_fire_actor (Utilities|Casting|CastToBP_WeaponFireActor Weapon))
  (bind _asbp_weapon_rifle_actor (Utilities|Casting|CastToBP_WeaponRifleActor _asbp_weapon_fire_actor))
  (Variables|Default|GetWeaponRifle
    (:then)
    (:else
      (bind _output_get (Variables|Default|SetWeaponRifle _asbp_weapon_rifle_actor))
      (Collision|SetActorEnableCollision _output_get false)
      (CallFunction|WeaponAttach _output_get "Skt_HideRifle"))))

(fn WeaponAttach
  (params (Weapon :type BP%20Weapon%20Actor%20Object%20Reference) (SocketName :type Name))
  (Transformation|AttachComponentToComponent Weapon (Variables|/Script/Engine.Character|GetMesh (Variables|Default|GetCharacter)) SocketName "KeepRelative" "KeepRelative" "KeepRelative" true))

(fn WeaponChange
  (params (Weapon :type BP%20Weapon%20Actor%20Object%20Reference))
  (bind _output_get (LocalVariables|SetL_Input_Weapon Weapon))
  (if (== _output_get (Variables|Default|GetWeaponCurrent))
    ;[1 1 1] Снять оружие
    (Variables|Default|SetWeaponCurrent 0)
    (CallFunction|WeaponAttach (LocalVariables|GetL_Input_Weapon) "Skt_HideRifle")
    (else
      (bind _weaponcurrent (Variables|Default|GetWeaponCurrent)
        (:then
          ;[1 1 1] Снять оружие
          (CallFunction|WeaponDrop _weaponcurrent)
          (bind _output_get_2 (Variables|Default|SetWeaponCurrent (LocalVariables|GetL_Input_Weapon)))
          (CallFunction|WeaponAttach _output_get_2 "Skt_CurWeapon"))
        (:else
          (bind _output_get_3 (Variables|Default|SetWeaponCurrent (LocalVariables|GetL_Input_Weapon)))
          (CallFunction|WeaponAttach _output_get_3 "Skt_CurWeapon"))))))

(fn WeaponDrop
  (params (Weapon :type BP%20Weapon%20Actor%20Object%20Reference))
  (bind _character (Variables|Default|GetCharacter))
  (Transformation|DetachFromComponent (Variables|/Game/Blueprints/Storage/BP_StorageActor.BP_StorageActor_C|GetDefaultSceneRoot Weapon) "KeepRelative" "KeepRelative" "KeepRelative" true)
  (Collision|SetActorEnableCollision Weapon false)
  (Transformation|SetActorLocation Weapon (+ (Transformation|GetActorLocation _character) (* (Transformation|GetActorForwardVector _character) 1e+02)) false false))

(fn -ItemWeaponAdd
  (params (ItemWeaponAdd :type BP%20Storage%20Actor%20Object%20Reference%20%28by%20ref%29))
  (Utilities|Array|Add (Variables|Default|GetItemsWeapon) ItemWeaponAdd))

(fn -ItemWeaponBullets
  (params (ItemBulletsAdd :type BP%20St%20Act%20Bullet%20Object%20Reference%20%28by%20ref%29))
  (LocalVariables|SetL_BulletsAdd ItemBulletsAdd)
  (bind _array_element (Utilities|Array|ForEachLoopwithBreak (Variables|Default|GetItemsBullets) :!label _label)
    (:LoopBody
      (if (== (Utilities|GetClass _array_element) (Utilities|GetClass (LocalVariables|GetL_BulletsAdd)))
        (LocalVariables|SetL_FindBullet _array_element)
        (goto _label Break)))
    (:Completed
      (LocalVariables|GetL_FindBullet
        (:then
          (Variables|/Game/Blueprints/Storage/Bullets/BP_St_Act_Bullet.BP_St_Act_Bullet_C|SetValue (LocalVariables|GetL_FindBullet) (+ (Variables|/Game/Blueprints/Storage/Bullets/BP_St_Act_Bullet.BP_St_Act_Bullet_C|GetValue (LocalVariables|GetL_BulletsAdd)) (Variables|/Game/Blueprints/Storage/Bullets/BP_St_Act_Bullet.BP_St_Act_Bullet_C|GetValue (LocalVariables|GetL_FindBullet))))
          (Actor|DestroyActor (LocalVariables|GetL_BulletsAdd)))
        (:else
          (Utilities|Array|Add (Variables|Default|GetItemsBullets) (LocalVariables|GetL_BulletsAdd))
          (Collision|SetActorEnableCollision (LocalVariables|GetL_BulletsAdd) false)
          (Transformation|SetActorLocation (LocalVariables|GetL_BulletsAdd) "0, 0, 0" false false)
          (Rendering|SetActorHiddenInGame (LocalVariables|GetL_BulletsAdd) false))))))

(fn -FindCurBullet
  (bind _weaponcurrent (Variables|Default|GetWeaponCurrent)
    (:then
      (bind _asbp_weapon_fire_actor (Utilities|Casting|CastToBP_WeaponFireActor _weaponcurrent)
        (:then
          (bind _array_element (Utilities|Array|ForEachLoopwithBreak (Variables|Default|GetItemsBullets) :!label _label)
            (:LoopBody
              (if (== (Utilities|GetClass _array_element) (Variables|/Game/Blueprints/Storage/Weapon/Fire/BP_WeaponFireActor.BP_WeaponFireActor_C|GetBullets_Type_Fire _asbp_weapon_fire_actor))
                (LocalVariables|SetL_Bullets _array_element)
                (goto _label Break)))
            (:Completed
              (bind _l_bullets (LocalVariables|GetL_Bullets)
                (:then
                  (return _l_bullets))
                (:else
                  (return 0))))))
        (:CastFailed
          (return 0))))
    (:else
      (return 0))))