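; BP_SpawnNPC is a world spawner that creates NPCs at random ground points inside its SpawnArea box.
; NewSpawnNPC marks it active and starts a delay timer for SpawnNPC, which spawns NPCClass above the point, passes on NavMesh and tracks the actor.
; GetRandomSpawnPoint line-traces down through the box with debug drawing, and also runs in the construction script.
; CheckNPCSpawn clears the timer and deactivates the spawner once MaxNPC is reached.
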(event EventBeginPlay)

(fn ConstructionScript
  (CallFunction|GetRandomSpawnPoint))

(fn SpawnNPC
  (bind _location (CallFunction|GetRandomSpawnPoint))
  (bind _returnvalue (Game|SpawnActorfromClass (Variables|Default|GetNPC_Class) (Math|Transform|MakeTransform (+ _location "0, 0,150.000000")) "Undefined" 0 0))
  (Variables|/Game/Blueprints/NPC/BP_NPC_Character.BP_NPC_Character_C|SetNavMesh _returnvalue (Variables|Default|GetNavMesh))
  (Utilities|Array|Add (Variables|Default|GetNPCs) _returnvalue)
  (CallFunction|CheckNPCSpawn))

(fn GetRandomSpawnPoint
  (bind _spawnarea (Variables|Default|GetSpawnArea))
  (bind _spawnarea_2 (Variables|Default|GetSpawnArea))
  (bind _returnvalue (Transformation|GetWorldLocation _spawnarea))
  (bind _returnvalue_2 (Components|Box|GetScaledBoxExtent _spawnarea_2))
  (bind (_x _y _z) (Math|Vector|BreakVector _returnvalue_2))
  (bind _returnvalue_3 (* _returnvalue_2 -1.0))
  (bind (_x_2 _y_2) (Math|Vector|BreakVector _returnvalue_3))
  (bind _returnvalue_4 (Math|Random|RandomFloatinRange _y_2 _y))
  (bind _returnvalue_5 (Math|Random|RandomFloatinRange _x_2 _x))
  (bind _returnvalue_6 (Math|Vector|MakeVector _returnvalue_5 _returnvalue_4 _z))
  (bind _returnvalue_7 (+ _returnvalue _returnvalue_6))
  (bind _outhit (Collision|LineTraceByChannel _returnvalue_7 (- _returnvalue_7 (Math|Vector|MakeVector 0.0 0.0 (* _z 2.0))) "TraceTypeQuery1" false 0 "ForDuration"))
  (return (.Location (Collision|BreakHitResult _outhit))))

(fn CheckNPCSpawn
  (if (<= (Variables|Default|GetMaxNPC) (Utilities|Array|Length (Variables|Default|GetNPCs)))
    (Utilities|Time|ClearandInvalidateTimerbyHandle (Variables|Default|GetTimer_SpawnNPC))
    (Variables|Default|SetIsActive false)))

(fn NewSpawnNPC
  (Variables|Default|SetIsActive true)
  (bind _returnvalue (Utilities|Time|SetTimerbyFunctionName 0 "SpawnNPC" (Variables|Default|GetSpawnDelay)))
  (Variables|Default|SetTimer_SpawnNPC _returnvalue))