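; BP_DayNightCircle drives a day-night cycle from a Time value on a 24-hour clock advanced by TimeSpeed.
; Each Tick updates the clock, refreshes the sky sphere's sun, pitches the directional light through a full turn and prints the time.
; Fog density uses clamped lerps, ramping up to MaxFog over hours 4–5 and back to zero over 20–21.
; The Construction Script runs the same update, minus the print.
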(event EventBeginPlay)

(event Collision|EventActorBeginOverlap
  (params (OtherActor :type Actor%20Object%20Reference)))

(event EventTick
  (params (DeltaSeconds :type Float%20%28single-precision%29))
  (CallFunction|-TimeCounter)
  (Default|UpdateSunDirection (Variables|Default|GetSkySphere))
  (CallFunction|-RotateDirLight)
  (CallFunction|-Fog)
  (Development|PrintString (Utilities|String|ToString(Float) (Variables|Default|GetTime)) true true "(R=0.000000,G=0.660000,B=1.000000,A=1.000000)" 0.0))

(fn ConstructionScript
  (CallFunction|-TimeCounter)
  (Default|UpdateSunDirection (Variables|Default|GetSkySphere))
  (CallFunction|-RotateDirLight)
  (CallFunction|-Fog))

(fn -TimeCounter
  (bind _output_get (Variables|Default|SetTime (+ (Variables|Default|GetTime) (* (Utilities|Time|GetWorldDeltaSeconds) (Variables|Default|GetTimeSpeed)))))
  (if (>= _output_get 24.0)
    (Variables|Default|SetTime 0.0)))

(fn -RotateDirLight
  (Transformation|SetActorRotation (Variables|Default|GetDirLight) (Math|Rotator|MakeRotator 0.0 (Math|Float|Lerp 9e+01 4.5e+02 (/ (Variables|Default|GetTime) 24.0)) 0.0)))

(fn -Fog
  (bind _time (Variables|Default|GetTime))
  (bind _maxfog (Variables|Default|GetMaxFog))
  (Class|ExponentialHeightFogComponent|SetFogDensity (Variables|/Script/Engine.ExponentialHeightFog|GetComponent (Variables|Default|GetFog)) (Math|Float|Max(Float) 0.0 (Math|Float|Min(Float) (Math|Float|SelectFloat (Math|Float|Lerp 0.0 _maxfog (- _time 4.0)) (Math|Float|Lerp _maxfog 0.0 (- _time 2e+01)) (< _time 5.0)) _maxfog))))