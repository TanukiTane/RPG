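; BP_Tree is a tree place actor that a character can start and stop an interaction with, built on a parent class that supplies the core behavior.
; Start runs the parent logic, waits one second less than DelayPlaceWait, then calls Stop on the same character, which defers to the parent.
; Tick calls Rotation on itself every frame, and the construction script only runs the parent's.
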(event Event-Start
  (params (Chatacter :type BP%20Main%20Chacter%20Object%20Reference))
  (|CallParentFunction Chatacter)
  (Utilities|FlowControl|Delay (- (Variables|Default|GetDelayPlaceWait) 1.0))
  (CallFunction|-Stop Chatacter))

(event Event-Stop
  (params (Chatacter :type BP%20Main%20Chacter%20Object%20Reference))
  (|CallParentFunction Chatacter))

(event EventTick
  (params (DeltaSeconds :type Float%20%28single-precision%29))
  (CallFunction|-Rotation self))

(fn ConstructionScript
  (|CallParentFunction))