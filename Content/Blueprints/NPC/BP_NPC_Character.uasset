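; NPC character that switches between Patrol and Combat states, showing the current one on an overhead status widget.
; BeginPlay stores a spawned rifle and ammo, and PawnSensing alarms the NPC on seeing a living player, retrying while animations play.
; Alarming draws the rifle and dispatches the target.
; Per-state data sets the widget and a timeline cooldown, which gates attack permission in Combat and puts the weapon away in Patrol.
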(event OnSeePawn(PawnSensing)
  (params (Pawn :type Pawn%20Object%20Reference))
  ;[1 0.04144 0.06134] OnSeePawn
  (bind _asbp_player_character (Utilities|Casting|CastToBP_PlayerCharacter Pawn))
  (bind _output_get (Variables|Default|SetGoal%20Player _asbp_player_character))
  (if (not (Variables|/Game/Blueprints/BP_MainChacter.BP_MainChacter_C|GetisDeath _output_get))
    (Attr|-isAlarmed)))

(event Custom|UpdateTimeline
  (params (IsReverse :type Boolean))
  (bind _self self)
  (bind _datacomp (Variables|Widget|GetDataComp))
  (bind _timelinecomponent (Variables|Default|GetTimelineComponent))
  (bind _maxtime (Utilities|Struct|BreakST_DataComponent _datacomp))
  (bind _returnvalue (Components|Timeline|GetPlaybackPosition _timelinecomponent))
  (bind _returnvalue_2 (Components|Timeline|GetTimelineLength _timelinecomponent))
  (bind _bp_storage_component (Variables|Default|GetBP_Storage_Component _self))
  (bind _returnvalue_3 (/ _returnvalue _returnvalue_2))
  ;[1 1 1] Condition to delay for begin attack
  (switch Utilities|FlowControl|Switch|SwitchonE_components (Utilities|Struct|BreakST_DataComponent (Variables|Widget|GetDataComp))
    (:NewEnumerator0
      (Widget|-WBaseColor "NewEnumerator0" :!label _label)
      (Components|Timeline|SetTimelineLength (Variables|Default|GetTimelineComponent) _maxtime)
      (Timeline|TimelineComponent PlayFromStart
        (:Update
          (bind _cooldownmaterial (Variables|/Game/UI/Widget/W_IconComponents.W_IconComponents_C|GetCoolDownMaterial (Variables|Widget|GetWidgetStatus))
            (:then
              (Rendering|Material|SetScalarParameterValue _cooldownmaterial "Percent" (Math|Float|SelectFloat (- 1.0 _returnvalue_3) _returnvalue_3 IsReverse) :!class /Script/Engine.MaterialInstanceDynamic)
              (Rendering|Material|SetVectorParameterValue _cooldownmaterial "Color" (Utilities|Struct|BreakST_DataComponent (Variables|Widget|GetDataComp)) :!class /Script/Engine.MaterialInstanceDynamic))
            (:else)))
        (:Finished
          (switch Utilities|FlowControl|Switch|SwitchonE_components (Utilities|Struct|BreakST_DataComponent (Variables|Widget|GetDataComp))
            (:NewEnumerator0
              (Widget|SetVisibility (Variables|Widget|GetWidgetStatus) "Hidden")
              (Variables|bool|SetisActivate-isPatrolling false)
              ;[1 1 1] NPC Clear weapon in hand
              (if (Variables|Default|GetIsCurWeapon self)
                (bind _weaponcurrent (Variables|/Game/Blueprints/Components/BP_Storage_Component.BP_Storage_Component_C|GetWeaponCurrent _bp_storage_component)
                  (:then
                    (Default|WeaponChange _bp_storage_component _weaponcurrent)
                    ;[1 1 1] Deactivate fast target attack
                    (Variables|Default|SetisAttackAllowed false))
                  (:else))))
            (:NewEnumerator1
              (Variables|Default|SetisAttackAllowed true)
              (Variables|bool|SetisActivate-isPatrolling true)
              (Widget|SetVisibility (Variables|Widget|GetWidgetStatus) "Visible")
              (if (not IsReverse)
                (Widget|-WBaseColor "NewEnumerator1")
                (bind _cooldownmaterial_2 (Variables|/Game/UI/Widget/W_IconComponents.W_IconComponents_C|GetCoolDownMaterial (Variables|Widget|GetWidgetStatus))
                  (:then
                    (Rendering|Material|SetScalarParameterValue _cooldownmaterial_2 "Percent" 0.0 :!class /Script/Engine.MaterialInstanceDynamic)
                    (if (Variables|Default|GetisDeath)
                      (Development|SetHiddeninGame (Variables|Default|GetWidget) true false)))
                  (:else))))))))
    (:NewEnumerator1
      (if (not (Math|Boolean|ANDBoolean (Variables|bool|GetisActivate-isPatrolling) true (not IsReverse)))
        (goto _label)
        (else
          (CallFunction|StopUpdateTimeLine)
          (Variables|Default|SetisAttackAllowed true))))))

(event Custom|Stop_UpdateTimeLine
  (Audio|Components|Audio|Stop (Variables|Default|GetTimelineComponent))
  (Widget|-WBaseColor "NewEnumerator1")
  (bind _cooldownmaterial (Variables|/Game/UI/Widget/W_IconComponents.W_IconComponents_C|GetCoolDownMaterial (Variables|Widget|GetWidgetStatus))
    (:then
      (Rendering|Material|SetScalarParameterValue _cooldownmaterial "Percent" 0.0 :!class /Script/Engine.MaterialInstanceDynamic)
      (if (Variables|Default|GetisDeath)
        (Development|SetHiddeninGame (Variables|Default|GetWidget) true false)))
    (:else)))

(event EventBeginPlay
  (bind _self self)
  ;[0.2705 0.2451 1] BeginPlay
  (|CallParentFunction)
  (Rendering|SetVisibility (Variables|Default|GetWidget) false false)
  (Variables|Widget|SetWidgetStatus (.AsW%20Icon%20Components (Utilities|Casting|CastToW_IconComponents (UserInterface|GetUserWidgetObject (Variables|Default|GetWidget)))))
  (bind _weapon_rifle (Variables|weapon|GetWeapon_Rifle)
    (:then
      _)
    (:else
      (bind _returnvalue (Game|SpawnActorfromClass "/Game/Blueprints/Storage/Weapon/Fire/Rifle/BP_WeaponRifleActor_SM_G36C-SF.BP_WeaponRifleActor_SM_G36C-SF_C" (Math|Transform|MakeTransform (Math|Vector|MakeVector 0.0 0.0 0.0) "0, 0, 0" "1,1,1") "Undefined" _self _self))
      (Variables|weapon|SetWeapon_Rifle _returnvalue)))
  ;;[1 1 1] Weapon_Rifle Add
  (Default|-ItemsAllAdd (Variables|Default|GetBP_Storage_Component) _weapon_rifle)
  (bind _returnvalue_2 (Game|SpawnActorfromClass (Variables|/Game/Blueprints/Storage/Weapon/Fire/BP_WeaponFireActor.BP_WeaponFireActor_C|GetBullets_Type_Fire _weapon_rifle) (Math|Transform|MakeTransform "0, 0, 0" "0, 0, 0" "1,1,1") "Undefined" _weapon_rifle self))
  (Variables|/Game/Blueprints/Storage/Bullets/BP_St_Act_Bullet.BP_St_Act_Bullet_C|SetValue _returnvalue_2 15)
  (Default|-ItemsAllAdd (Variables|Default|GetBP_Storage_Component) _returnvalue_2))

(event Collision|EventActorBeginOverlap
  (params (OtherActor :type Actor%20Object%20Reference)))

(event EventTick
  (params (DeltaSeconds :type Float%20%28single-precision%29)))

(fn ConstructionScript
  (|CallParentFunction))

(fn -isAlarmed
  (bind _self self)
  (bind _bp_storage_component (Variables|Default|GetBP_Storage_Component _self))
  (if (not (Variables|Default|GetisDeath self))
    ;[1 1 1] If animation playing yet called this function after 0.1 sec
    (if (not (Variables|Default|GetIsPlayingAnimation self))
      (if (not (Variables|bool|GetisAlarming))
        (Utilities|FlowControl|Sequence
          (:then_0
            (Variables|Default|SetIsRunning true)
            (Variables|bool|SetisAlarming true)
            (Variables|bool|SetisPatrolling false))
          (:then_1
            ;[1 1 1] Add Rifle to NPC, if there is no weapon in hands
            (if (not (Variables|Default|GetIsCurWeapon self))
              (bind _weaponrifle (Variables|/Game/Blueprints/Components/BP_Storage_Component.BP_Storage_Component_C|GetWeaponRifle _bp_storage_component)
                (:then
                  (Default|WeaponChange _bp_storage_component _weaponrifle))
                (:else))))
          (:then_2
            ;[1 1 1] Update component and call to combat component from dispatcher. If yete is no target npc begin patrolling
            (bind _goal_player (Variables|Default|GetGoal%20Player)
              (:then
                (Widget|-WUpdate "NewEnumerator1")
                (Default|Call+Alarmed _goal_player))
              (:else
                (Attr|-isPatrolling))))))
      (else
        (Utilities|Time|SetTimerbyFunctionName 0 "-isAlarmed" 0.1)))))

(fn -isPatrolling
  ;[1 1 1] Проверка на смерть
  (if (not (Variables|Default|GetisDeath self))
    (if (not (Variables|bool|GetisPatrolling))
      (Variables|Default|SetIsRunning false)
      (Variables|bool|SetisAlarming false)
      (Variables|bool|SetisPatrolling true)
      (Variables|Default|SetGoal%20Player 0)
      (Widget|-WUpdate "NewEnumerator0"))))

(fn -ParamComponent
  (params (ComponentActiveStatus :type E_components%20Enum :default "NewEnumerator0"))
  (bind _array_element (Utilities|Array|ForEachLoopwithBreak (Variables|Widget|GetComponentsMaster))
    (:LoopBody
      (if (Utilities|Enum|Equal(Enum) (.Component (Utilities|Struct|BreakST_DataComponent _array_element)) ComponentActiveStatus)
        (return true _array_element)))
    (:Completed
      (return false ""))))

(fn -WUpdate
  (params (ComponentActiveStatus :type E_components%20Enum :default "NewEnumerator0"))
  (bind (_sucsses _array_element) (Widget|-ParamComponent ComponentActiveStatus))
  (if _sucsses
    (Variables|Widget|SetDataComp _array_element)
    (Variables|/Game/UI/Widget/W_IconComponents.W_IconComponents_C|SetStatus (Variables|Widget|GetWidgetStatus) (Utilities|Struct|BreakST_DataComponent (Variables|Widget|GetDataComp)))
    (Widget|SetVisibility (Variables|/Game/UI/Widget/W_IconComponents.W_IconComponents_C|GetIcon (Variables|Widget|GetWidgetStatus)) "Visible")
    (Rendering|SetVisibility (Variables|Default|GetWidget) false false)
    (Class|Image|SetBrush (Variables|/Game/UI/Widget/W_IconComponents.W_IconComponents_C|GetIcon (Variables|Widget|GetWidgetStatus)) (Utilities|Struct|MakeSlateBrush "(X=32.000000,Y=32.000000)" "(Left=0.000000,Top=0.000000,Right=0.000000,Bottom=0.000000)" "(SpecifiedColor=(R=1.000000,G=1.000000,B=1.000000,A=1.000000),ColorUseRule=UseColor_Specified)" (Utilities|Struct|BreakST_DataComponent (Variables|Widget|GetDataComp)) "Image" "NoTile" "NoMirror"))
    (Rendering|SetVisibility (Variables|Default|GetWidget) true false)
    (CallFunction|UpdateTimeline false)
    (else
      (Attr|-isPatrolling))))

(fn -WBaseColor
  (params (Selection :type E_components%20Enum :default "NewEnumerator0"))
  (switch Utilities|FlowControl|Switch|SwitchonE_components Selection
    (:NewEnumerator0
      ;[1 1 1] Default Value
      (Variables|/Game/UI/Widget/W_IconComponents.W_IconComponents_C|SetBase%20Color (Variables|Widget|GetWidgetStatus) (Utilities|Struct|MakeSlateColor "(R=1.000000,G=1.000000,B=1.000000,A=1.000000)") :!label _label))
    (:NewEnumerator1
      ;[1 1 1] Color from component
      (bind (_sucsses _array_element) (Widget|-ParamComponent Selection))
      (if _sucsses
        (Variables|/Game/UI/Widget/W_IconComponents.W_IconComponents_C|SetBase%20Color (Variables|Widget|GetWidgetStatus) (Utilities|Struct|MakeSlateColor (Utilities|Struct|BreakST_DataComponent _array_element)))
        (else
          (goto _label))))))