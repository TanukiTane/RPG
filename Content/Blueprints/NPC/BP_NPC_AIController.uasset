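; AI controller for NPCs that switches between roaming and combat behaviour.
; On possess it caches the instigator as BP_NPC_Character, initialises the roaming and combat components, starts roaming and binds to the NPC's Alarmed event.
; Alarmed stores the goal player, stops roaming and starts combat.
; Patrol reverses this by stopping combat, restarting roaming and calling the NPC's isPatrolling.
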(event EventPossess
  (params (PossessedPawn :type Pawn%20Object%20Reference))
  (CallFunction|-Init))

(fn ConstructionScript)

(fn -Init
  ;[1 1 1] Set NPC
  (bind _asbp_npc_character (Utilities|Casting|CastToBP_NPC_Character (Game|GetInstigator)))
  (Variables|Default|SetNPC _asbp_npc_character)
  ;[1 1 1] Roaming Init
  (Default|-Init (Variables|Default|GetBP_Roaming_Components))
  ;[1 1 1] Roaming Start
  (Default|-Start (Variables|Default|GetBP_Roaming_Components))
  ;[1 1 1] Combat Component Init
  (Default|-Init (Variables|Default|GetBP_Combat_component))
  (CallFunction|-BindEvents))

(fn -Alarmed
  (params (GoalPlayer :type BP%20Player%20Character%20Object%20Reference))
  (Variables|Default|SetGoalPlayer GoalPlayer)
  (if (Variables|/Game/Blueprints/NPC/Components/BP_Roaming_Components.BP_Roaming_Components_C|GetRoaming (Variables|Default|GetBP_Roaming_Components))
    (Default|-Stop (Variables|Default|GetBP_Roaming_Components)))
  (Default|-Start (Variables|Default|GetBP_Combat_component)))

(fn -Patrol
  (Default|-Stop (Variables|Default|GetBP_Combat_component))
  (Default|-Start (Variables|Default|GetBP_Roaming_Components))
  (Default|-isPatrolling (Variables|Default|GetNPC)))

(fn -BindEvents
  ;[1 1 1] BindEvent to +Alarmed
  (EventDispatchers|BindEventto+Alarmed (Variables|Default|GetNPC) (EventDispatchers|CreateEvent :!event -Alarmed)))