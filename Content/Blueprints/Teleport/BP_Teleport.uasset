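; BP_Teleport is a portal actor that teleports actors entering its Box trigger to a randomly chosen linked portal.
; Box overlap starts a three-second Delay, then moves the overlapping actor to a random ConnectedPortals entry's root location with zeroed rotation, without rechecking the overlap.
; The PortalNumber comparison has no effect, since both SelectInt options resolve to the array's last index.
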(event OnComponentBeginOverlap(Box)
  (params (OverlappedComponent :type Primitive%20Component%20Object%20Reference) (OtherActor :type Actor%20Object%20Reference) (OtherComp :type Primitive%20Component%20Object%20Reference) (OtherBodyIndex :type Integer) (bFromSweep :type Boolean) (SweepResult :type Hit%20Result%20Structure%20%28by%20ref%29))
  (bind _connectedportals (Variables|Default|GetConnectedPortals))
  (bind _returnvalue (Utilities|Array|Length _connectedportals))
  (bind _returnvalue_2 (- _returnvalue 1))
  ;[1 1 1] Teleport Function
  (Utilities|FlowControl|Delay 3.0)
  (Transformation|Teleport OtherActor (Transformation|GetWorldLocation (Variables|/Script/Engine.Actor|GetRootComponent (Utilities|Array|Get(acopy) (Variables|Default|GetConnectedPortals) (Math|Random|RandomIntegerinRange 0 (Math|Integer|SelectInt _returnvalue_2 _returnvalue_2 (< _returnvalue (Variables|Default|GetPortalNumber))))))) "0, 0, 0"))

(event EventBeginPlay)

(event Collision|EventActorBeginOverlap
  (params (OtherActor :type Actor%20Object%20Reference)))

(event EventTick
  (params (DeltaSeconds :type Float%20%28single-precision%29)))

(fn ConstructionScript)