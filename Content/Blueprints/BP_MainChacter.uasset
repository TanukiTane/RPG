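; BP_MainChacter is a base character Blueprint handling storage, health, movement speed and ragdoll death.
; BeginPlay initializes the storage and health components.
; Tick runs Sprint on both iron-sights branches, setting sprint or run speed; a separate IronSights function sets walk speed but is not called here.
; IsDeath flags death, disables player input, and, for player or NPC AI controllers, starts a timer enabling mesh ragdoll physics.
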(event EventTick
  (params (DeltaSeconds :type Float%20%28single-precision%29))
  (if (Variables|Default|GetIsIronSights)
    (CallFunction|-Sprint)
    (else
      (CallFunction|-Sprint))))

(event EventBeginPlay
  ;[0.2917 0.1303 1] BeginPlay
  (CallFunction|-Init))

(fn ConstructionScript)

(fn -Init
  ;[1 1 1] Storage Init
  (Default|-Init (Variables|Default|GetBP_Storage_Component))
  ;[1 1 1] Health Init
  (Default|-Init (Variables|Default|GetBP_HealthComponent)))

(fn -Sprint
  (if (Variables|Default|GetIsSprint)
    (Variables|/Script/Engine.CharacterMovementComponent|SetMaxWalkSpeed (Variables|Character|GetCharacterMovement self) (Variables|Default|GetSprint))
    (else
      (Variables|/Script/Engine.CharacterMovementComponent|SetMaxWalkSpeed (Variables|Character|GetCharacterMovement self) (Variables|Default|GetRun)))))

(fn -IronSights
  (if (Variables|Default|GetIsIronSights)
    (Variables|/Script/Engine.CharacterMovementComponent|SetMaxWalkSpeed (Variables|Character|GetCharacterMovement self) (Variables|Default|GetWalk))
    (else
      (Variables|/Script/Engine.CharacterMovementComponent|SetMaxWalkSpeed (Variables|Character|GetCharacterMovement self) (Variables|Default|GetRun)))))

(fn -IsDeath
  (Variables|Death|SetisDeath true)
  (bind _asplayer_controller (Utilities|Casting|CastToPlayerController (Game|GetInstigatorController))
    (:then
      (Input|DisableInput _asplayer_controller 0))
    (:CastFailed
      (Utilities|Casting|CastToBP_NPC_AIController (Game|GetInstigatorController))))
  (Utilities|Time|SetTimerbyFunctionName 0 "-EnableRagdoll" 1.0))

(fn -EnableRagdoll
  (Collision|SetCollisionEnabled (Variables|Collision|GetCapsuleComponent) "NoCollision")
  (Physics|SetSimulatePhysics (Variables|Character|GetMesh) true)
  (Collision|SetCollisionEnabled (Variables|Character|GetMesh) "QueryAndPhysics")
  (Collision|SetCollisionResponsetoAllChannels (Variables|Character|GetMesh) "ECR_Block"))