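; BP_WeaponFireActor is a firearm actor that fires projectiles from its magazine and reloads from the owning character's storage.
; IsFire spends a round, spawning the configured bullet and a small explosion effect at the muzzle, or calls Reload when empty.
; Reloading is guarded by a flag and delayed, then IsReload tops up the magazine from BP_MainChacter's current bullet stack, capped at capacity, and deducts the rounds taken.
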(event Custom|_Reload
  (bind _asbp_main_chacter (Utilities|Casting|CastToBP_MainChacter (Components|GetOwner)))
  (Variables|Default|SetL_Bullets (Default|-FindCurBullet (Variables|/Game/Blueprints/BP_MainChacter.BP_MainChacter_C|GetBP_Storage_Component _asbp_main_chacter)))
  (bind _l_bullets (Variables|Default|GetL_Bullets)
    (:then
      (if (Math|Boolean|ANDBoolean (not (Variables|Default|GetBulletReload)) (< (Variables|Bullets|GetBulletsCurValue) (Variables|Bullets|GetBulletsMaxValue)) (> (Variables|/Game/Blueprints/Storage/Bullets/BP_St_Act_Bullet.BP_St_Act_Bullet_C|GetValue _l_bullets) 0))
        (Variables|Default|SetBulletReload true)
        (Utilities|FlowControl|Delay (Variables|Bullets|GetBulletsDelayReload self))
        (CallFunction|-IsReload)))
    (:else)))

(fn ConstructionScript
  (|CallParentFunction))

(fn -IsFire
  (params (Target :type Vector%20%28by%20ref%29))
  (bind (_spawn _rotation) (|Location))
  ;[1 1 1] Spawn Bullets
  (LocalVariables|SetL_Target Target)
  (if (> (Variables|Bullets|GetBulletsCurValue self) 0)
    (Math|Integer|DecrementInt (Variables|Bullets|GetBulletsCurValue self)
      (:%20%20
        (Game|SpawnActorfromClass (Variables|Static|GetBullets_TypeSpawn) _spawn "AlwaysSpawn" self (Game|GetInstigator))
        (Effects|SpawnEmitteratLocation "/Game/Visual/StarterContent/Particles/P_Explosion.P_Explosion" (Transformation|GetWorldLocation (Variables|Default|GetBulletsSpawnLocation)) _rotation "0.050000,0.050000,0.050000")))
    (else
      (CallFunction|Reload))))

(fn -IsReload
  (bind _asbp_main_chacter (Utilities|Casting|CastToBP_MainChacter (Components|GetOwner))
    (:then
      (LocalVariables|SetL_Bullet (Default|-FindCurBullet (Variables|/Game/Blueprints/BP_MainChacter.BP_MainChacter_C|GetBP_Storage_Component _asbp_main_chacter)))
      (bind _l_bullet (LocalVariables|GetL_Bullet)
        (:then
          (if (> (Variables|/Game/Blueprints/Storage/Bullets/BP_St_Act_Bullet.BP_St_Act_Bullet_C|GetValue _l_bullet) 0)
            (LocalVariables|SetL_BulletValue (+ (Variables|Bullets|GetBulletsCurValue) (Variables|/Game/Blueprints/Storage/Bullets/BP_St_Act_Bullet.BP_St_Act_Bullet_C|GetValue (LocalVariables|GetL_Bullet))))
            (Variables|/Game/Blueprints/Storage/Bullets/BP_St_Act_Bullet.BP_St_Act_Bullet_C|SetValue (LocalVariables|GetL_Bullet) (Math|Integer|Max(Integer) 0 (- (LocalVariables|GetL_BulletValue) (Variables|Bullets|GetBulletsMaxValue))))
            (Variables|Bullets|SetBulletsCurValue (Math|Integer|SelectInt (Variables|Bullets|GetBulletsMaxValue) (LocalVariables|GetL_BulletValue) (> (LocalVariables|GetL_BulletValue) (Variables|Bullets|GetBulletsMaxValue))))
            (Variables|Default|SetBulletReload false)
            (else
              (Variables|Default|SetBulletReload false))))
        (:else
          (Variables|Default|SetBulletReload false))))
    (:CastFailed
      (Variables|Default|SetBulletReload false))))